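; BP_Teste is an actor, apparently a test, that keeps its root pointed at the InnerShell actor.
; BeginPlay snaps the root to the look-at rotation, then combines the StaticMesh's world rotation with the negated initial rotation to offset that snap.
; Tick recomputes the look-at rotation every frame, so the child mesh turns with the root while tracking InnerShell.
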(event `self.ReceiveTick`
  (params (DeltaSeconds :type "Float (single-precision)"))
  (bind _defaultsceneroot (`self.DefaultSceneRoot`))
  (`SceneComponent.K2_SetWorldRotation` _defaultsceneroot (`KismetMathLibrary.FindLookAtRotation` (`SceneComponent.K2_GetComponentLocation` _defaultsceneroot) (`SceneComponent.K2_GetComponentLocation` (`Actor.RootComponent` (`self.InnerShell`)))) false false))

(event `self.ReceiveBeginPlay`
  (bind _staticmesh (`self.StaticMesh`))
  (bind _defaultsceneroot (`self.DefaultSceneRoot`))
  (bind _output_get (set `self.InitialRotator` (`KismetMathLibrary.FindLookAtRotation` (`SceneComponent.K2_GetComponentLocation` _defaultsceneroot) (`SceneComponent.K2_GetComponentLocation` (`Actor.RootComponent` (`self.InnerShell`))))))
  (`SceneComponent.K2_SetWorldRotation` _defaultsceneroot _output_get false false)
  (`SceneComponent.K2_SetWorldRotation` _staticmesh (`KismetMathLibrary.ComposeRotators` (`SceneComponent.K2_GetComponentRotation` _staticmesh) (`KismetMathLibrary.NegateRotator` (`self.InitialRotator`))) false false))

(fn `UserConstructionScript`
  (locals (InnerSheel :type "StaticMeshActor Object Reference")))