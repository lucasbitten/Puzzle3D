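; Construction-script Blueprint that distributes copies of a chosen mesh in an evenly spaced row from the actor toward an EndPoint offset, likely for skylights or pillars.
; It adds scaled static mesh components under PillarStartPoint, stepping along local X by the offset's length divided by Amount, provided that spacing is large enough.
; PillarStartPoint is then yawed toward EndPoint, ignoring pitch; the event graph is empty.
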(fn `UserConstructionScript`
  (bind _returnvalue (`self.K2_GetActorLocation`))
  (bind _amount (`self.Amount`))
  (bind _returnvalue_2 (/ (`KismetMathLibrary.VSize` (`self.EndPoint`)) _amount))
  (`StaticMeshComponent.SetStaticMesh` (`self.PillarStartPoint`) (`self.MeshToSpawn`))
  (if (> (`KismetMathLibrary.Round` (- _returnvalue_2 1.0)) 0)
    ;[1 1 1] Loop Body
    (for _index (range (+ (`KismetMathLibrary.FTrunc` _amount) 1))
      (bind _returnvalue_3 (`AddComponent|NODE_AddStaticMeshComponent-0` :`RelativeTransform` (`KismetMathLibrary.MakeTransform` (0.0 0.0 0.0) (struct) (`KismetMathLibrary.Conv_DoubleToVector` (`self.Pillar_Scale`)))))
      (`SceneComponent.K2_AttachToComponent` _returnvalue_3 (`self.PillarStartPoint`) "None" "KeepRelative" "KeepRelative" "KeepRelative" true)
      (`SceneComponent.K2_SetRelativeLocation` _returnvalue_3 (`KismetMathLibrary.MakeVector` (* _index _returnvalue_2)) false false)
      (`StaticMeshComponent.SetStaticMesh` _returnvalue_3 (`self.MeshToSpawn`)))
    (`SceneComponent.K2_SetWorldRotation` (`self.PillarStartPoint`) (`KismetMathLibrary.MakeRotator` 0.0 0.0 (.yaw (`KismetMathLibrary.FindLookAtRotation` _returnvalue (+ _returnvalue (`self.EndPoint`))))) false false)))