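; Plant distribution Blueprint that lays out a row of randomly chosen static meshes at construction time.
; The construction script divides the EndPoint vector's length by Amount for spacing, then adds mesh components along PlantStartPoint's local X axis.
; Each gets a random mesh from MeshToSpawn, clamped random scale and vertical jitter.
; The yaw rotation toward EndPoint is disconnected, so only that vector's length affects the layout.
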(fn `UserConstructionScript`
  (bind _returnvalue (`KismetMathLibrary.RandomFloat`))
  (bind _amount (`self.Amount`))
  (bind _outitem (`KismetArrayLibrary.Array_Random` (`self.MeshToSpawn`)))
  (bind _returnvalue_2 (`KismetMathLibrary.FClamp` _returnvalue (`self.ScaleMin`) 2.0))
  (bind _returnvalue_3 (`KismetMathLibrary.FTrunc` _amount))
  (bind _returnvalue_4 (/ (`KismetMathLibrary.VSize` (`self.EndPoint`)) _amount))
  (bind _returnvalue_5 (* (- _returnvalue 0.5) 25.0))
  (`StaticMeshComponent.SetStaticMesh` (`self.PlantStartPoint`) _outitem)
  (if (> (`KismetMathLibrary.Round` (- _returnvalue_4 1.0)) 0)
    ;[1 1 1] Loop Body
    (for _index (range (+ _returnvalue_3 1))
      (bind _returnvalue_6 (`AddComponent|NODE_AddStaticMeshComponent-0` :`RelativeTransform` (`KismetMathLibrary.MakeTransform` (`KismetMathLibrary.MakeVector` 0.0 0.0 _returnvalue_5) (struct) (`KismetMathLibrary.MakeVector` _returnvalue_2 _returnvalue_2 _returnvalue_2))))
      (`SceneComponent.K2_AttachToComponent` _returnvalue_6 (`self.PlantStartPoint`) "None" "KeepRelative" "KeepRelative" "KeepRelative" true)
      (`SceneComponent.K2_SetRelativeLocation` _returnvalue_6 (`KismetMathLibrary.MakeVector` (* _index _returnvalue_4) 0.0 _returnvalue_5) false false)
      (`StaticMeshComponent.SetStaticMesh` _returnvalue_6 _outitem)
      (for _ (range (+ _returnvalue_3 1))
        _))))