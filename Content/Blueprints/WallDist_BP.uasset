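; WallDist_BP is a construction-script placement tool that repeats a chosen static mesh, such as a wall pillar, at even intervals over a set distance.
; PillarStartPoint shows the first mesh, and a loop attaches copies along its local X, spaced by EndPoint's length divided by Amount, if that spacing is large enough.
; Yaw rotation toward EndPoint is disconnected, so only the vector's length matters.
; The event graph is empty.
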(fn `UserConstructionScript`
  (bind _amount (`self.Amount`))
  (bind _returnvalue (/ (`KismetMathLibrary.VSize` (`self.EndPoint`)) _amount))
  (`StaticMeshComponent.SetStaticMesh` (`self.PillarStartPoint`) (`self.MeshToSpawn`))
  (if (> (`KismetMathLibrary.Round` (- _returnvalue 1.0)) 0)
    ;[1 1 1] Loop Body
    (for _index (range (+ (`KismetMathLibrary.FTrunc` _amount) 1))
      (bind _returnvalue_2 (`AddComponent|NODE_AddStaticMeshComponent-0`))
      (`SceneComponent.K2_AttachToComponent` _returnvalue_2 (`self.PillarStartPoint`) "None" "KeepRelative" "KeepRelative" "KeepRelative" true)
      (`SceneComponent.K2_SetRelativeLocation` _returnvalue_2 (`KismetMathLibrary.MakeVector` (* _index _returnvalue)) false false)
      (`StaticMeshComponent.SetStaticMesh` _returnvalue_2 (`self.MeshToSpawn`)))))