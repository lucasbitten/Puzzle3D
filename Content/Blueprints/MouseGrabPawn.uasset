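; Player pawn for a 3D puzzle game that orbits and zooms around a PuzzleModel and drags pieces with the mouse.
; Tick traces under the cursor, gliding the held piece over the surface, oriented toward inverse-distance-weighted hits from inner-mesh traces.
; An optional hint material changes color with distance to the correct position.
; Camera limits come from the model, sphere traces correct zoom penetration, and distance drives FOV and post-process.
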(event `self.ReceiveTick`
  (params (DeltaSeconds :type "Float (single-precision)"))
  (bind (_raystart _rayend) (`self.CreateRayFromMouseLocation`))
  (bind _currentpiececomponent (`self.CurrentPieceComponent`))
  ;[1 1 1] Movement
  (set `self.Delta` DeltaSeconds)
  (if (`self.GrabMode`)
    (if (and (`KismetSystemLibrary.IsValid` (`self.CurrentPieceComponent`)) (`self.CanMovePiece`))
      (bind (_outhit _returnvalue) (`KismetSystemLibrary.LineTraceSingle` _raystart _rayend "TraceTypeQuery4" true))
      (if _returnvalue
        (`self.SetPointToLookAt`)
        (`SceneComponent.K2_SetWorldRotation` (`self.CurrentPieceComponent`) (`KismetMathLibrary.RInterpTo` (`SceneComponent.K2_GetComponentRotation` (`self.CurrentPieceComponent`)) (`KismetMathLibrary.FindLookAtRotation` (`SceneComponent.K2_GetComponentLocation` (`self.CurrentPieceComponent`)) (`self.PointToLookAt`)) (`self.Delta`) 20.0) false false)
        (bind (_bblockinghit _binitialoverlap _time _distance _location _impactpoint _normal _impactnormal) (`GameplayStatics.BreakHitResult` _outhit))
        (`SceneComponent.K2_SetWorldLocation` _currentpiececomponent (`KismetMathLibrary.VInterpTo` (`SceneComponent.K2_GetComponentLocation` _currentpiececomponent) (+ _impactpoint (* _impactnormal (`self.MovementDistanceOffset`))) (`self.Delta`) (`self.PieceMovementInterpSpeed`)) false false)
        (`PuzzlePieceParentComponent.RestorePieceInitialRelativeRotation` (`self.CurrentPieceComponent`))
        (`self.SetMaterialColor`)
        (else
          (`SceneComponent.K2_SetWorldLocation` (`self.CurrentPieceComponent`) (`self.CalculatePositionOutsideModel`) false false)))
      (`self.UpdateDesiredArmLength`)
      (else
        (`self.UpdateDesiredArmLength` :!label _label)))
    (else
      (goto _label)))
  (set `SpringArmComponent.TargetArmLength` (`KismetMathLibrary.FInterpTo` (`SpringArmComponent.TargetArmLength` (`self.SpringArm`)) (`self.DesiredArmLength`) (`self.Delta`) (`self.CameraInterpSpeed`)) (`self.SpringArm`)))

(event `InputAxisKey|MouseX`
  (params (AxisValue :type "Float (single-precision)"))
  (bind (_returnvalue_roll _returnvalue_pitch _returnvalue_yaw) (`KismetMathLibrary.BreakRotator` (`self.GetControlRotation`)))
  ;[1 1 1] Mouse Movement
  (if (not (`self.GrabMode`))
    (if (`GI_Puzzle.InvertX` (`self.PuzzleGameInstance`))
      (`self.AddControllerYawInput` AxisValue)
      (else
        (`self.AddControllerYawInput` (* AxisValue -1.0))))
    (`Controller.SetControlRotation` (`GameplayStatics.GetPlayerController` 0) (`KismetMathLibrary.MakeRotator` 0.0 _returnvalue_pitch _returnvalue_yaw))
    (`self.UpdateDesiredArmLength` :!label _label_2)
    (`self.Set Camera FOV`)))

(event `InputAxisKey|MouseY`
  (params (AxisValue :type "Float (single-precision)"))
  ;[1 1 1] Mouse Movement
  (if (`self.GrabMode`)
    _
    (elif (`GI_Puzzle.InvertY` (`self.PuzzleGameInstance`))
      (`self.HandleVerticalMovement` (* AxisValue -1.0))
      (goto _label_2)
      (else
        (`self.HandleVerticalMovement` AxisValue)))))

(event `self.ReceiveBeginPlay`
  ;[1 1 1] BeginPlay
  (set `self.CameraSpringArm` (`self.SpringArm`))
  (bind _asgm_puzzle_mode (cast `GM_PuzzleMode` (`GameplayStatics.GetGameMode`)))
  (bind _returnvalue (`GameplayStatics.GetActorOfClass` "/Script/Puzzle3D.PuzzleModel"))
  (`/Engine/EditorBlueprintResources/StandardMacros.IsValid` _returnvalue
    (:`Is Valid`
      (`self.ModelLoaded` _returnvalue))
    (:`Is Not Valid`
      (add `GM_PuzzleMode.OnModelLoaded` _asgm_puzzle_mode (`|CreateDelegate` :!event `OnModelLoaded`))))
  (add `GM_PuzzleMode.OnModelExploded` _asgm_puzzle_mode (`|CreateDelegate` :!event `OnModelExploded`))
  (bind _returnvalue_2 (`KismetMaterialLibrary.CreateDynamicMaterialInstance` "/Game/Art/Materials/Outline.Outline" "Outline_Hint"))
  (bind _output_get (set `self.HintMaterial` _returnvalue_2))
  (bind _returnvalue_3 (`MaterialInstanceDynamic.K2_GetVectorParameterValue` _output_get "InteriorColor"))
  (set `self.InitialMaterialColor` _returnvalue_3))

(event `OnModelLoaded`
  ;[1 1 1] BeginPlay
  (bind _returnvalue (`GameplayStatics.GetActorOfClass` "/Script/Puzzle3D.PuzzleModel"))
  (`self.ModelLoaded` _returnvalue))

(event `Key|MouseScrollUp`
  (params (Key :type "Key Structure"))
  ;[1 1 1] MouseWheel
  (:`Pressed`
    (set `self.ArmLengthIncrement` (- (`self.ArmLengthIncrement`) (`self.CameraZoomSpeed`)))
    (`self.Set Camera FOV` :!label _label_3)))

(event `OnModelExploded`
  ;[1 1 1] Board Placement
)

(event `Key|MouseScrollDown`
  (params (Key :type "Key Structure"))
  ;[1 1 1] MouseWheel
  (:`Pressed`
    (set `self.ArmLengthIncrement` (+ (`self.ArmLengthIncrement`) (`self.CameraZoomSpeed`)))
    (goto _label_3)))

(fn `CalculateDistanceFromCorrectPosition`
  (returns (ReturnValue :type "Float (double-precision)"))
  (bind _currentpiececomponent (`self.CurrentPieceComponent`))
  (return (`KismetMathLibrary.Vector_Distance` (`SceneComponent.K2_GetComponentLocation` _currentpiececomponent) (`PuzzlePieceParentComponent.GetParentInitialWorldPositionWithOffset` _currentpiececomponent))))

(fn `CalculatePositionOutsideModel`
  (returns (ReturnValue :type "Vector Structure"))
  (bind (_worldlocation _worlddirection) (`PlayerController.DeprojectMousePositionToWorld` (`GameplayStatics.GetPlayerController` 0)))
  (return (+ _worldlocation (* _worlddirection (`self.PieceInWorldDistanceFromCamera`)))))

(fn `CalculateSpringArmTargetArmLength`
  (params (CanMoveBack :type Boolean))
  (returns (ArmLengthIncrement :type "Float (double-precision)"))
  (locals (Direction :type "Vector Structure" :default (0.0 0.0 0.0)) (ShellLocation :type "Vector Structure" :default (0.0 0.0 0.0)) (DesiredCameraLocation :type "Vector Structure" :default (0.0 0.0 0.0)) (FinalArmLengthIncrement :type "Float (double-precision)"))
  (bind _currentmodel (`self.CurrentModel`))
  (bind _returnvalue (`KismetMathLibrary.Vector_Distance` (`local.DesiredCameraLocation`) (`local.ShellLocation`)))
  (bind _targetarmlength (`SpringArmComponent.TargetArmLength` (`self.SpringArm`)))
  (bind _shell (`PuzzleModel.Shell` _currentmodel))
  (`/Engine/EditorBlueprintResources/StandardMacros.IsValid` _currentmodel
    (:`Is Valid`
      (`/Engine/EditorBlueprintResources/StandardMacros.IsValid` _shell
        (:`Is Valid`
          (set `local.ShellLocation` (`SceneComponent.K2_GetComponentLocation` _shell))
          (set `local.Direction` (`KismetMathLibrary.GetDirectionUnitVector` (`SceneComponent.K2_GetComponentLocation` (`self.Camera`)) (`local.ShellLocation`)))
          (set `local.DesiredCameraLocation` (+ (`local.ShellLocation`) (* (+ (`SpringArmComponent.TargetArmLength` (`self.SpringArm`)) (`self.ArmLengthIncrement`)) (`local.Direction`) -1.0)))
          (bind (_outhit _returnvalue_2) (`KismetSystemLibrary.SphereTraceSingle` (+ (* (`KismetMathLibrary.Vector_Distance` (`local.DesiredCameraLocation`) (`local.ShellLocation`)) (`local.Direction`) -2.0) (`local.ShellLocation`)) (`local.ShellLocation`) (`self.MaxZoomOffset`) "TraceTypeQuery4" true))
          (if _returnvalue_2
            (bind _returnvalue_3 (`KismetMathLibrary.Vector_Distance` (`.Location` (`GameplayStatics.BreakHitResult` _outhit)) (`local.ShellLocation`)))
            (if (> _returnvalue_3 _returnvalue)
              (if (<= (`self.ArmLengthIncrement`) 0.0)
                (bind _returnvalue_4 (- _returnvalue_3 _returnvalue))
                (bind _returnvalue_5 (+ _targetarmlength _returnvalue_4 -5.0))
                (bind _returnvalue_6 (- _targetarmlength _returnvalue_5))
                (if (>= _returnvalue_6 0.0)
                  (set `local.FinalArmLengthIncrement` 0.0)
                  (`KismetSystemLibrary.PrintString` "aqui 1")
                  (else
                    (`KismetSystemLibrary.PrintString` "aqui 2")
                    (set `local.FinalArmLengthIncrement` (`KismetMathLibrary.Abs` _returnvalue_6) :!label _label)))
                (else
                  (`KismetSystemLibrary.PrintString` (`KismetStringLibrary.Concat_StrStr` "How Much Camera is Inside: " (`KismetStringLibrary.Conv_DoubleToString` _returnvalue_4) "\\n Corrected arm length: " (`KismetStringLibrary.Conv_DoubleToString` _returnvalue_5) "\\n Arm Length difference: " (`KismetStringLibrary.Conv_DoubleToString` _returnvalue_6)))
                  (goto _label)))
              (if (`local.CanMoveBack`)
                (return (`local.FinalArmLengthIncrement`))
                (elif (not (> (`local.FinalArmLengthIncrement`) (`SpringArmComponent.TargetArmLength` (`self.SpringArm`))))
                  (return (`local.FinalArmLengthIncrement`))))
              (else
                (return (`self.ArmLengthIncrement`))))))))))

(fn `CalculateWeightedPoint`
  (returns (Output_Get :type "Vector Structure"))
  (return (`KismetMathLibrary.MakeVector` (/ (`self.SumX`) (`KismetMathLibrary.FMax` (`self.TotalWeight`) 1e-05)) (/ (`self.SumY`) (`KismetMathLibrary.FMax` (`self.TotalWeight`) 1e-05)) (/ (`self.SumZ`) (`KismetMathLibrary.FMax` (`self.TotalWeight`) 1e-05)))))

(fn `CreateRayFromMouseLocation`
  (returns (RayStart :type "Vector Structure") (RayEnd :type "Vector Structure"))
  (bind (_worldlocation _worlddirection) (`PlayerController.DeprojectMousePositionToWorld` (`GameplayStatics.GetPlayerController` 0)))
  (return _worldlocation (+ _worldlocation (* _worlddirection 10000.0))))

(fn `DeselectPieceComponent`
  (params (PieceComponent :type "PuzzlePieceParentComponent Object Reference"))
  (`PrimitiveComponent.SetMaterial` (`PuzzlePieceParentComponent.GetPieceMesh` PieceComponent) 1 (`self.OriginalMaterial`)))

(fn `GetRemovingFinalParentPosition`
  (returns (ReturnValue :type "Vector Structure"))
  (bind _currentpiececomponent (`self.CurrentPieceComponent`))
  (bind _returnvalue (`PuzzlePieceParentComponent.GetOffsetDistance` _currentpiececomponent))
  (return (+ (`SceneComponent.K2_GetComponentLocation` _currentpiececomponent) (* (* _returnvalue (`SceneComponent.GetForwardVector` _currentpiececomponent)) -1.0))))

(fn `Handle Piece Touched`
  (params (TouchedComponent :type "SceneComponent Object Reference"))
  (bind _returnvalue (`PrimitiveComponent.GetMaterial` (`PuzzlePieceParentComponent.GetPieceMesh` (`self.CurrentPieceComponent`)) 1))
  (bind _aspuzzle_piece_parent_component (cast `PuzzlePieceParentComponent` (`SceneComponent.GetAttachParent` TouchedComponent)))
  (if (`PuzzlePieceParentComponent.GetIsLocked` _aspuzzle_piece_parent_component)
    (`KismetSystemLibrary.PrintString` "Locked")
    (else
      (set `self.CurrentPieceComponent` _aspuzzle_piece_parent_component)
      (if (not (`KismetSystemLibrary.IsValid` (`self.OriginalMaterial`)))
        (`/Engine/EditorBlueprintResources/StandardMacros.IsValid` _returnvalue
          (:`Is Valid`
            (bind _returnvalue_2 (`MaterialInterface.GetBaseMaterial` _returnvalue))
            (set `self.OriginalMaterial` _returnvalue_2))
          (:`Is Not Valid`
            _)))
      (bind _asgi_puzzle (cast `GI_Puzzle` (`GameplayStatics.GetGameInstance`)))
      (if (`GI_Puzzle.ShowHints` _asgi_puzzle)
        (`PrimitiveComponent.SetMaterial` (`PuzzlePieceParentComponent.GetPieceMesh` (`self.CurrentPieceComponent`)) 1 (`self.HintMaterial`)))
      (set `self.CanMovePiece` false))))

(fn `HandleVerticalMovement`
  (params (InputPin :type "Float (single-precision)"))
  (locals (Input :type "Float (single-precision)"))
  (bind _springarm (`self.SpringArm`))
  (bind (_returnvalue_x _returnvalue_y _returnvalue_z) (`KismetMathLibrary.BreakVector` (`SceneComponent.K2_GetComponentLocation` (`self.Camera`))))
  (bind (_returnvalue_x_2 _returnvalue_y_2 _returnvalue_z_2) (`KismetMathLibrary.BreakVector` (`SceneComponent.K2_GetComponentLocation` _springarm)))
  (bind (_returnvalue_x_3 _returnvalue_y_3 _returnvalue_z_3) (`KismetMathLibrary.BreakVector` (`SceneComponent.K2_GetComponentLocation` (`self.Camera`))))
  (set `local.Input` InputPin)
  (if (> _returnvalue_z (+ (`PuzzleModel.ModelTopZ` (`self.CurrentModel`)) (`self.zTopOffset`)))
    (`self.AddControllerPitchInput` (`local.Input`))
    (elif (> _returnvalue_z_3 (`PuzzleModel.ModelBottomZ` (`self.CurrentModel`)))
      (`SceneComponent.K2_SetWorldLocation` _springarm (`KismetMathLibrary.MakeVector` _returnvalue_x_2 _returnvalue_y_2 (+ _returnvalue_z_2 (* (`local.Input`) (`self.CameraZSpeed`)))) false false :!label _label)
      (`self.AddControllerPitchInput` (* (`local.Input`) 0.5))
      (elif (> (`local.Input`) 0.0)
        (goto _label)))))

(fn `IsPieceCloseToCamera`
  (returns (ReturnValue :type Boolean))
  (return (< (`KismetMathLibrary.Vector_Distance` (`SceneComponent.K2_GetComponentLocation` (`self.CurrentPieceComponent`)) (`SceneComponent.K2_GetComponentLocation` (`self.Camera`))) (`self.PieceInWorldDistanceFromCamera`))))

(fn `ModelLoaded`
  (params (CurrentModel :type "PuzzleModel Object Reference"))
  (bind _currentmodel (`self.CurrentModel`))
  (bind _output_get (set `self.CurrentModel` CurrentModel))
  (set `self.SphereArrays` (`PuzzleModel.GetInnerMeshComponents` _output_get))
  (set `self.MovementDistanceOffset` (`PuzzleModel.GetOffsetDistance` _currentmodel))
  (`SceneComponent.K2_SetWorldLocation` (`self.SpringArm`) (`SceneComponent.K2_GetComponentLocation` (`PuzzleModel.Shell` _currentmodel)) false false)
  (`self.Set Camera Variables`))

(fn `ResetValues`
  (set `self.TotalWeight` 0.0)
  (set `self.SumX` 0.0)
  (set `self.SumY` 0.0)
  (set `self.SumZ` 0.0))

(fn `Set Camera FOV`
  (bind _returnvalue (/ (- (`KismetMathLibrary.Vector_Distance` (`SceneComponent.K2_GetComponentLocation` (`self.Camera`)) (0.0 -20.0 150.0)) (`self.MinCameraDistance`)) (- (`self.MaxCameraDistance`) (`self.MinCameraDistance`))))
  (set `PostProcessComponent.Settings` (make `PostProcessSettings` :`AutoExposureMinBrightness` -3.0 :`AutoExposureMaxBrightness` 6.0 :`DepthOfFieldFocalDistance` (`KismetMathLibrary.Lerp` 95.0 400.0 _returnvalue)) (`self.PostProcess_Blurry`))
  (`CameraComponent.SetPostProcessBlendWeight` (`self.Camera`) _returnvalue)
  (`CameraComponent.SetFieldOfView` (`self.Camera`) (`KismetMathLibrary.Lerp` 53.0 48.0 _returnvalue)))

(fn `Set Camera Variables`
  (bind _currentmodel (`self.CurrentModel`))
  (`/Engine/EditorBlueprintResources/StandardMacros.IsValid` _currentmodel
    (:`Is Valid`
      (set `self.MinCameraDistance` (`PuzzleModel.MinCameraDistance` _currentmodel))
      (set `self.MaxCameraDistance` (`PuzzleModel.MaxCameraDistance` (`self.CurrentModel`)))
      (set `self.MaxZoomOffset` (`PuzzleModel.MaxZoomOffset` (`self.CurrentModel`)))
      (set `self.ArmLengthIncrement` (`PuzzleModel.ArmLengthIncrement` (`self.CurrentModel`)))
      (set `self.DesiredArmLength` (`PuzzleModel.DesiredArmLength` (`self.CurrentModel`)))
      (set `self.CameraInterpSpeed` (`PuzzleModel.CameraInterpSpeed` (`self.CurrentModel`)))
      (set `self.CameraZoomSpeed` (`PuzzleModel.CameraZoomSpeed` (`self.CurrentModel`)))
      (set `self.CameraZSpeed` (`PuzzleModel.CameraZSpeed` (`self.CurrentModel`))))))

(fn `SetMaterialColor`
  (`MaterialInstanceDynamic.SetVectorParameterValue` (`self.HintMaterial`) "InteriorColor" (`KismetMathLibrary.LinearColorLerp` (`self.InitialMaterialColor`) (`self.CloseMaterialColor`) (`KismetMathLibrary.MapRangeClamped` (`self.CalculateDistanceFromCorrectPosition`) (`self.CloseDistanceRange`) 0.0 0.0 1.0))))

(fn `SetPointToLookAt`
  (locals (NewLocalVar :type "EDrawDebugTrace Enum" :default "None"))
  (bind _returnvalue (`SceneComponent.K2_GetComponentLocation` (`self.CurrentPieceComponent`)))
  (`self.ResetValues`)
  (for _array_element (`self.SphereArrays`)
    (bind _returnvalue_2 (`SceneComponent.K2_GetComponentLocation` _array_element))
    (if (<= (`KismetMathLibrary.Vector_Distance` _returnvalue _returnvalue_2) (`self.MaxRaycastLenght`))
      (bind (_outhit _returnvalue_3) (`KismetSystemLibrary.LineTraceSingle` :`Start` _returnvalue :`End` _returnvalue_2 :`TraceChannel` "TraceTypeQuery4" :`bTraceComplex` true :`bIgnoreSelf` false :`DrawTime` 0.0))
      (if _returnvalue_3
        (bind (_bblockinghit _binitialoverlap _time _distance _location _impactpoint) (`GameplayStatics.BreakHitResult` _outhit))
        (`self.SetSumPositionsAndTotalWeight` _distance _impactpoint))))
  (bind _output_get (`self.CalculateWeightedPoint`))
  (bind _output_get_2 (set `self.PointToLookAt` _output_get))
  (`KismetSystemLibrary.DrawDebugSphere` _output_get_2 1.0 12 (struct :`R` 1.0 :`G` 1.0 :`B` 1.0 :`A` 1.0) 0.0 0.1))

(fn `SetSumPositionsAndTotalWeight`
  (params (DistanceFromPiece :type "Float (double-precision)") (ImpactPoint :type "Vector Structure"))
  (bind _returnvalue (/ 1.0 (`KismetMathLibrary.FMax` (`KismetMathLibrary.MultiplyMultiply_FloatFloat` (`KismetMathLibrary.FMax` DistanceFromPiece 1.0) (`self.DistancePower`)) 0.001)))
  (set `self.TotalWeight` (+ (`self.TotalWeight`) _returnvalue))
  (set `self.SumX` (+ (* (.x ImpactPoint) _returnvalue) (`self.SumX`)))
  (set `self.SumY` (+ (* (.y ImpactPoint) _returnvalue) (`self.SumY`)))
  (set `self.SumZ` (+ (* (.z ImpactPoint) _returnvalue) (`self.SumZ`))))

(fn `UpdateDesiredArmLength`
  (bind _armlengthincrement (`self.CalculateSpringArmTargetArmLength` true))
  (set `self.DesiredArmLength` (`KismetMathLibrary.FClamp` (+ _armlengthincrement (`SpringArmComponent.TargetArmLength` (`self.SpringArm`))) (`self.MinCameraDistance`) (`self.MaxCameraDistance`)))
  (set `self.ArmLengthIncrement` 0.0))

(fn `UpdateMaxValues`
  (params (ImpactPoint :type "Vector Structure"))
  (if (>= (.x ImpactPoint) 0.0)
    _
    (elif (>= (.y ImpactPoint) 0.0)
      _
      (elif (>= (.z ImpactPoint) 0.0)
        _))))

(fn `UpdateMinValues`
  (params (ImpactPoint :type "Vector Structure"))
  (if (<= (.x ImpactPoint) 0.0)
    _
    (elif (<= (.y ImpactPoint) 0.0)
      _
      (elif (<= (.z ImpactPoint) 0.0)
        _))))

(fn `UserConstructionScript`
  (bind _outactors (`GameplayStatics.GetAllActorsOfClassWithTag` "/Script/Engine.PostProcessVolume" "CamControl"))
  (set `self.PostProc_volume` (`KismetArrayLibrary.Array_Random` _outactors)))